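; Demolisher is a hex-map entity Blueprint whose ability demolishes wall tiles.
; It overrides OnAbilityOrder, first requiring the parent check to pass, then requiring the target hex to be a wall with no actors on it.
; A valid target becomes a floor tile through the hex map with a mesh update, while an invalid one prints a red error and returns false.
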(event EventBeginPlay
  (|CallParentFunction))

(event Collision|EventActorBeginOverlap
  (params (OtherActor :type Actor%20Object%20Reference)))

(event EventTick
  (params (DeltaSeconds :type Float%20%28single-precision%29))
  (|CallParentFunction DeltaSeconds))

(fn ConstructionScript
  (|CallParentFunction))

(fn OnAbilityOrder
  (params (TargetHex :type Hex%20Vector%20Structure))
  (bind _currenthexmap (Utilities|GetHexMap))
  (bind _returnvalue (Class|HexMap|GetDataatHex _currenthexmap TargetHex))
  (bind _validuse (|CallParentFunction TargetHex))
  (if _validuse
    (if (and (== (Utilities|Set|Length (Variables|/Script/HexGameFramework.HexTileData|GetActorsOnTile _returnvalue)) 0) (Variables|/Script/HexGameFramework.HexTileData|GetIsWall _returnvalue))
      (Class|HexMap|AddorChangeHex _currenthexmap TargetHex "/Game/Blueprints/Tiles/Tile_Floor.Tile_Floor_C" true)
      (return true)
      (else
        (Development|PrintText "Invalid Location!" true true "(R=1.000000,G=0.000000,B=0.000000,A=1.000000)")
        (return false)))))