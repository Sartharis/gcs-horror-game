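; TileProp is a prop on the hex tile grid that can spawn a Blob on its own tile.
; SpawnBlob runs only if CanSpawnBlob is set and no blob has spawned yet, then marks it spawned so it happens once.
; The spawn plays a slime particle effect at EmitterPoint and a sound at the prop's location.
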(event Custom|SpawnBlob
  (if (and (not (Variables|Default|GetSpawnedBlob)) (Variables|Default|GetCanSpawnBlob))
    (Utilities|SpawnActoronTile "/Game/Blueprints/Entities/Blob.Blob_C" (CallFunction|GetActorHexPosition))
    (Variables|Default|SetSpawnedBlob true)
    (Effects|SpawnEmitteratLocation "/Game/StarterContent/Particles/P_SpawnSlime.P_SpawnSlime" (Transformation|GetWorldLocation (Variables|Default|GetEmitterPoint)))
    (Audio|PlaySoundatLocation "/Game/Sound/Spawn_Cue.Spawn_Cue" (Transformation|GetActorLocation))))

(event EventBeginPlay
  (|CallParentFunction))

(event Collision|EventActorBeginOverlap
  (params (OtherActor :type Actor%20Object%20Reference)))

(event EventTick
  (params (DeltaSeconds :type Float%20%28single-precision%29)))

(fn ConstructionScript
  (|CallParentFunction))