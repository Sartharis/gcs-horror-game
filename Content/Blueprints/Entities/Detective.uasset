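; Detective is an entity whose ability scans the hexes around a target for enemies.
; Its OnAbilityOrder override runs the parent check, then looks through the actors on each hex map tile within ScanRadius for an AggroEnemy.
; The first match ends the scan, and the result is reported only as a printed debug message, returning true whether or not an enemy is found.
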(event EventBeginPlay
  (|CallParentFunction))

(event Collision|EventActorBeginOverlap
  (params (OtherActor :type Actor%20Object%20Reference)))

(event EventTick
  (params (DeltaSeconds :type Float%20%28single-precision%29))
  (|CallParentFunction DeltaSeconds))

(fn ConstructionScript
  (|CallParentFunction))

(fn OnAbilityOrder
  (params (TargetHex :type Hex%20Vector%20Structure))
  (bind _validuse (|CallParentFunction TargetHex))
  (if _validuse
    (for _array_element (Class|HexFunctionLibrary|HexinRadius TargetHex (Variables|Default|GetScanRadius))
      (bind _result (Utilities|Set|ToArray (Variables|/Script/HexGameFramework.HexTileData|GetActorsOnTile (Class|HexMap|GetDataatHex (Utilities|GetHexMap) _array_element))))
      (for _array_element_2 _result
        (Utilities|Casting|CastToAggroEnemy _array_element_2)
        (Development|PrintString "ENEMY DETECTED!!!" true true "(R=1.000000,G=0.000000,B=0.000000,A=1.000000)")
        (return true)))
    (Development|PrintString "No enemies detected." true true "(R=1.000000,G=0.000000,B=0.000000,A=1.000000)")
    (return true)))