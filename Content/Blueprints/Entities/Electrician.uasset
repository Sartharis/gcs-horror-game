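; Electrician entity for a hex-map game whose ability repairs broken activation switches.
; OnAbilityOrder runs the parent check, then looks through the actors on the target hex for an ActivationSwitch.
; The first switch found decides the result: a broken one is fixed and returns true, otherwise it prints "Nothing broken!" and returns false.
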(event EventBeginPlay
  (|CallParentFunction))

(event Collision|EventActorBeginOverlap
  (params (OtherActor :type Actor%20Object%20Reference)))

(event EventTick
  (params (DeltaSeconds :type Float%20%28single-precision%29))
  (|CallParentFunction DeltaSeconds))

(fn ConstructionScript
  (|CallParentFunction))

(fn OnAbilityOrder
  (params (TargetHex :type Hex%20Vector%20Structure))
  (bind _validuse (|CallParentFunction ""))
  (if _validuse
    (bind _result (Utilities|Set|ToArray (Variables|/Script/HexGameFramework.HexTileData|GetActorsOnTile (Class|HexMap|GetDataatHex (Utilities|GetHexMap) TargetHex))))
    (for _array_element _result
      (bind _asactivation_switch (Utilities|Casting|CastToActivationSwitch _array_element))
      (if (Variables|/Game/Blueprints/Entities/ActivationSwitch.ActivationSwitch_C|GetBroken _asactivation_switch)
        (Variables|/Game/Blueprints/Entities/ActivationSwitch.ActivationSwitch_C|SetBroken _asactivation_switch false)
        (return true)
        (else
          (Development|PrintText "Nothing broken!" true true "(R=1.000000,G=0.000000,B=0.000000,A=1.000000)")
          (return false))))
    (Development|PrintText "Nothing broken!" true true "(R=1.000000,G=0.000000,B=0.000000,A=1.000000)")
    (return false)))