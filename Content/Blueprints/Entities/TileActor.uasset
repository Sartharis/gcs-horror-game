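; TileActor is a base actor that occupies a hex tile on the HexMap and tracks its hex position.
; Its construction script finds an overlapping HexMap via SnapCollision, snaps RootMesh to the nearest hex and stores it; BeginPlay moves the root there and registers the actor.
; ChangeHexPosition re-registers and moves the actor, updates its HexLightComponents and fires OnLightUpdate, which is empty here, with the tile's lit state.
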(event Custom|OnLightUpdate
  (params (IsLit :type Boolean)))

(event EventBeginPlay
  (bind _rootmesh (Variables|Default|GetRootMesh))
  ;[1 1 1] Prepare the actor for regular gameplay by positioning its components correctly
  (Collision|SetCollisionEnabled (Variables|Default|GetSnapCollision) "NoCollision") ; We turn off the collsion, since we only use it in the construction script
  (Class|HexMap|RegisterActortoHex (Variables|/Script/HexGameFramework.HexGameFrameworkGameModeBase|GetCurrentHexMap (Utilities|GetHexGameMode)) (Variables|Default|GetHexPosition) self)
  (Transformation|SetWorldLocation (Variables|Default|GetDefaultSceneRoot) (Transformation|GetWorldLocation _rootmesh) false false)
  (Transformation|SetRelativeLocation _rootmesh "0, 0, 0" false false))

(fn ConstructionScript
  ;[1 1 1] Tile snapping and initial position setting
  (bind _outactors (Collision|ComponentOverlapActors (Variables|Default|GetSnapCollision) (Transformation|GetActorTransform) (Utilities|Array|MakeArray "ObjectTypeQuery2") "/Game/Blueprints/HexMap/HexMap.HexMap_C"))
  (Transformation|SetWorldLocation (Variables|Default|GetRootMesh) (Class|HexMap|HexVectortoPoint (.AsHex%20Map (Utilities|Casting|CastToHexMap (Utilities|Array|Get(acopy) _outactors))) (Class|HexMap|PointtoHexVector (.AsHex%20Map (Utilities|Casting|CastToHexMap (Utilities|Array|Get(acopy) _outactors))) (Transformation|GetWorldLocation (Variables|Default|GetDefaultSceneRoot)))) false false)
  (Variables|Default|SetHexPosition (Class|HexMap|PointtoHexVector (.AsHex%20Map (Utilities|Casting|CastToHexMap (Utilities|Array|Get(acopy) _outactors))) (Transformation|GetWorldLocation (Variables|Default|GetDefaultSceneRoot)))))

(fn ChangeHexPosition
  (params (NewPosition :type Hex%20Vector%20Structure))
  (bind _currenthexmap (Utilities|GetHexMap))
  (bind _self self)
  (Class|HexMap|UnregisterActorfromHex _currenthexmap (Variables|Default|GetHexPosition) _self)
  (Class|HexMap|RegisterActortoHex _currenthexmap NewPosition _self)
  (bind _output_get (Variables|Default|SetHexPosition NewPosition))
  (Transformation|SetActorLocation (Class|HexMap|HexVectortoPoint _currenthexmap _output_get) false false)
  (for _array_element (Actor|GetComponentsByClass "/Script/HexGameFramework.HexLightComponent")
    (Class|HexLightComponent|SetLightPosition _array_element (Variables|Default|GetHexPosition)))
  (CallFunction|OnLightUpdate (Class|HexMap|IsTileLitUp (Utilities|GetHexMap) _output_get)))

(fn GetActorHexPosition
  (return (Variables|Default|GetHexPosition)))