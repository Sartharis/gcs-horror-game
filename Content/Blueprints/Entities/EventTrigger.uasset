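; EventTrigger is a hex-grid trigger actor that gathers the actors on tiles within a radius of its own hex.
; Tick calls UpdateNearbyActors, which rebuilds NearbyActors from hex map data, firing OnOverlap and disabling tick inside the per-hex loop.
; OnOverlap is an empty hook for acting on the found actors.
; GetNearbyActorsofClass refreshes the list and compares classes, but does nothing with matches.
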(event Custom|Update%20Nearby%20Actors
  ;[1 1 1] Update Array of Actors within Trigger
  (Utilities|Array|Clear (Variables|Default|GetNearby%20Actors))
  (for _array_element (Class|HexFunctionLibrary|HexinRadius (CallFunction|GetActorHexPosition) (Variables|Default|GetRadius))
    (bind _result (Utilities|Set|ToArray (Variables|/Script/HexGameFramework.HexTileData|GetActorsOnTile (Class|HexMap|GetDataatHex (Utilities|GetHexMap) _array_element))))
    (for _array_element_2 _result
      (Utilities|Array|Add (Variables|Default|GetNearby%20Actors) _array_element_2))
    (CallFunction|OnOverlap (Variables|Default|GetNearby%20Actors))
    (Actor|Tick|SetActorTickEnabled false)))

(event Custom|Get%20Nearby%20Actors%20of%20Class
  (params (Class :type Actor%20Class%20Reference))
  ;[1 1 1] Get Nearby Actors of Some Class
  (CallFunction|UpdateNearbyActors)
  (for _array_element (Variables|Default|GetNearby%20Actors)
    (if (== (Utilities|GetClass _array_element) Class)
      _)))

(event Custom|On%20Overlap
  (params (Actors :type Array%20of%20Actor%20Object%20References))
  ;[1 1 1] Function Performed on Overlapping Actors
)

(event EventBeginPlay
  (|CallParentFunction))

(event Collision|EventActorBeginOverlap
  (params (OtherActor :type Actor%20Object%20Reference)))

(event EventTick
  (params (DeltaSeconds :type Float%20%28single-precision%29))
  ;[1 1 1] Update Every Tick
  (CallFunction|UpdateNearbyActors)
  (for _array_element (Variables|Default|GetNearby%20Actors)
    _))

(fn ConstructionScript
  (|CallParentFunction))