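; Player-controlled character for a turn-based hex-map game, with selection, action-point movement, a ranged ability, an inventory and death or resurrection.
; The Turn component refreshes action points and the ability, while emissive material swaps show turn and selection state.
; Orders move the character or interact with its own hex, and ability orders only range-check and spend the ability.
; Finished moves pick up items; death hides the character, drops items and leaves the turn manager.
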(event TurnActivateDelegate(Turn)
  ;[1 1 1] Selection texture effects
  (Rendering|Material|SetMaterial (Variables|Default|GetRootMesh) 0 "/Game/ColorEmissiveMaterial_Green.ColorEmissiveMaterial_Green")
  (Variables|Default|SetCurrentActionPoints (Variables|Default|GetMaxActionPoints))
  (Variables|Default|SetAbilityUp true))

(event TurnEndDelegate(Turn)
  ;[1 1 1] Selection texture effects
)

(event Custom|OnSelected
  ;[1 1 1] Selection texture effects
  (Rendering|Material|SetMaterial (Variables|Default|GetRootMesh) 0 "/Game/ColorEmissiveMaterial_Yellow.ColorEmissiveMaterial_Yellow")
  (Variables|Default|SetSelected true))

(event Custom|OnUnselected
  ;[1 1 1] Selection texture effects
  (Rendering|Material|SetMaterial (Variables|Default|GetRootMesh) 0 "/Game/ColorEmissiveMaterial.ColorEmissiveMaterial")
  (Variables|Default|SetSelected false))

(event Custom|OnEndTurnOrder
  ;[1 1 1] End Turn
  (Class|TurnComponent|EndTurn (Variables|Default|GetTurn))
  (Default|UnselectAll (Utilities|GetPlayerTileController)))

(event Custom|OnAbilitySelect
  ;[1 1 1] Using Ability Toggle
  (if (Variables|Default|GetAbilityUp)
    (bind _output_get (Variables|Default|SetUsingAbility (not (Variables|Default|GetUsingAbility))))
    (if _output_get
      (Development|PrintString "Using Ability" true true "(R=0.995000,G=0.000000,B=0.000000,A=1.000000)")
      (else
        (Development|PrintString "Canceled Ability" true true "(R=1.000000,G=0.000000,B=0.005000,A=1.000000)")))
    (else
      (Development|PrintString "No Ability!" true true "(R=1.000000,G=0.000000,B=0.000000,A=1.000000)"))))

(event EventOnMoveEnd
  ;[1 1 1] End of Movement Actions
  (|CallParentFunction)
  (bind _result (Utilities|Set|ToArray (Variables|/Script/HexGameFramework.HexTileData|GetActorsOnTile (Class|HexMap|GetDataatHex (Utilities|GetHexMap) (CallFunction|GetActorHexPosition)))))
  (for _array_element _result
    (bind _asitem (Utilities|Casting|CastToItem _array_element))
    (if (not (Variables|/Game/Blueprints/Entities/Item.Item_C|GetisHeld _asitem))
      (Default|PickedUp _asitem self)
      (Utilities|Array|Add (Variables|Default|GetInventory) _asitem))))

(event EventKill
  ;[1 1 1] Dying and Ressurecting
  (Variables|Default|SetDied true)
  (Development|SetHiddeninGame (Variables|Default|GetRootMesh) true true)
  (Class|TurnComponent|RemovefromTurnManager (Variables|Default|GetTurn))
  (Class|HexLightComponent|ToggleLight (Variables|Default|GetHexLight) false)
  (for _array_element (Variables|Default|GetInventory)
    (Default|Drop _array_element)
    (Utilities|Array|Clear (Variables|Default|GetInventory))
    (Utilities|Casting|CastToHorrorBaseGamemode (Game|GetGameMode))))

(event EventRessurect
  ;[1 1 1] Dying and Ressurecting
  (Variables|Default|SetDied false)
  (Development|SetHiddeninGame (Variables|Default|GetRootMesh) false true)
  (Class|TurnComponent|AddtoTurnManager (Variables|Default|GetTurn) true)
  (Class|HexLightComponent|ToggleLight (Variables|Default|GetHexLight) true))

(fn ConstructionScript
  (|CallParentFunction))

(fn CanbeSelected
  (return (and (Class|TurnComponent|IsinTurn (Variables|Default|GetTurn)) (not (Variables|Default|GetDied)))))

(fn OnAbilityOrder
  (params (TargetHex :type Hex%20Vector%20Structure))
  (if (Variables|Default|GetUsingAbility)
    (if (Variables|Default|GetAbilityUp)
      (if (<= (Class|HexFunctionLibrary|HDist TargetHex (CallFunction|GetActorHexPosition)) (Variables|Default|GetAbilityRadius))
        (Variables|Default|SetAbilityUp false)
        (Variables|Default|SetUsingAbility false)
        (return true)
        (else
          (Development|PrintString "Out of range!" true true "(R=1.000000,G=0.000000,B=0.000000,A=1.000000)")))
      (else
        (Development|PrintText "No ability!" true true "(R=1.000000,G=0.000000,B=0.000000,A=1.000000)")))
    (return false)))

(fn OnActionOrder
  (params (TargetHex :type Hex%20Vector%20Structure))
  (if (> (Utilities|Array|Length (Variables|Default|GetMovePath)) 0)
    (return false false "")
    (elif (Class|HexFunctionLibrary|EqualHexVectorHexVector TargetHex (CallFunction|GetActorHexPosition))
      (bind _result (Utilities|Set|ToArray (Variables|/Script/HexGameFramework.HexTileData|GetActorsOnTile (Class|HexMap|GetDataatHex (Utilities|GetHexMap) TargetHex))))
      (for _array_element _result
        (bind _asiinteractable (Utilities|Casting|CastToIInteractable _array_element))
        (bind _canbeinteractedwith (Default|CanbeInteractedwith _asiinteractable))
        (if _canbeinteractedwith
          (Default|OnInteraction _asiinteractable)))
      (return true false "")
      (elif (Variables|Default|GetUsingAbility)
        (return false false "")
        (else
          (bind (_canmove _movepath _movepointsused_) (CallFunction|StartMovetoPoint TargetHex (Variables|Default|GetCurrentActionPoints)))
          (Variables|Default|SetCurrentActionPoints (- (Variables|Default|GetCurrentActionPoints) _movepointsused_))
          (return true _canmove (Utilities|Array|Get(acopy) _movepath (Utilities|Array|LastIndex _movepath))))))))

(fn GetActorstoIgnore
  (return (Variables|Default|GetActorsToIgnoreBlockFrom)))

(fn IsDead
  (return (Variables|Default|GetDied)))