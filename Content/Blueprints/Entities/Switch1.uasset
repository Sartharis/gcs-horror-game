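; Switch1 is an interactable switch entity that activates a list of other actors.
; Each interaction flips its On state and calls OnActivate on every entry in ActorsToActivate whose CanBeActivated check passes, whether switching on or off.
; It accepts interaction while it is off, or in either state when Toggleable, so a non-toggleable switch cannot be turned back off through interaction.
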(event EventOnInteraction
  (Variables|Default|SetOn (not (Variables|Default|GetOn)))
  (for _array_element (Variables|Default|GetActorsToActivate)
    (bind _canbeactivated (Default|CanbeActivated _array_element))
    (if _canbeactivated
      (Default|OnActivate _array_element))))

(fn ConstructionScript)

(fn CanbeInteractedwith
  (return (or (Variables|Default|GetToggleable) (not (Variables|Default|GetOn)))))