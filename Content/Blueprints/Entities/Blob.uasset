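; Blob is a turn-based hex-grid creature that weakens attackable actors it lands on, then screams and destroys itself.
; Each turn it shakes and moves one point toward a random hex on or beside the nearest living PlayerCharacter if within two hexes, otherwise wanders to a random neighbour.
; Light updates show or hide its root mesh.
; Splat swaps it for a splat prop with a random sound, and destruction removes it from the turn manager.
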(event TurnActivateDelegate(Turn)
  (bind _hexposition (CallFunction|GetActorHexPosition))
  (bind _nexttarget (CallFunction|ChooseTarget))
  (bind _hexposition_2 (Default|GetActorHexPosition _nexttarget))
  (bind _returnvalue (Class|HexFunctionLibrary|HexRing _hexposition 1))
  (bind _returnvalue_2 (Class|HexFunctionLibrary|HexinRadius _hexposition_2 1))
  (if (Variables|Default|GetCanMove)
    (CallFunction|Shake 5.0 0.6)
    (bind _canmove (CallFunction|StartMovetoPoint (select (< (Class|HexFunctionLibrary|HDist _hexposition _hexposition_2) 3) (Utilities|Array|Get(acopy) _returnvalue_2 (Math|Random|RandomIntegerinRange 0 (- (Utilities|Array|Length _returnvalue_2) 1))) (Utilities|Array|Get(acopy) _returnvalue (Math|Random|RandomIntegerinRange 0 (- (Utilities|Array|Length _returnvalue) 1)))) 1))
    (if _canmove
      (Utilities|WaitUntilMoveEnded
        (:Move%20Done
          _))))
  (Utilities|FlowControl|Delay 0.1)
  (Class|TurnComponent|EndTurn (Variables|Default|GetTurn)))

(event TurnEndDelegate(Turn))

(event EventOnMoveEnd
  (bind _result (Utilities|Set|ToArray (Variables|/Script/HexGameFramework.HexTileData|GetActorsOnTile (Class|HexMap|GetDataatHex (Utilities|GetHexMap) (CallFunction|GetActorHexPosition)))))
  (for _array_element _result
    (bind _asiattackable (Utilities|Casting|CastToIAttackable _array_element))
    (Default|Weaken _asiattackable)
    (Audio|PlaySoundatLocation "/Game/Sound/Gasp_Quick_Female_KB_04_SCREAM_LIBRARY_BRFX-004.Gasp_Quick_Female_KB_04_SCREAM_LIBRARY_BRFX-004" (Transformation|GetActorLocation))
    (Actor|DestroyActor)))

(event EventOnLightUpdate
  (params (IsLit :type Boolean))
  (Development|SetHiddeninGame (Variables|Default|GetRootMesh) (not IsLit) false))

(event EventBeginPlay
  (|CallParentFunction))

(event EventDestroyed
  (|CallParentFunction)
  (Class|TurnComponent|RemovefromTurnManager (Variables|Default|GetTurn)))

(event EventTick
  (params (DeltaSeconds :type Float%20%28single-precision%29))
  (|CallParentFunction DeltaSeconds))

(fn ConstructionScript
  (|CallParentFunction))

(fn ChooseTarget
  (bind _hexposition (CallFunction|GetActorHexPosition))
  (bind _outactors (Actor|GetAllActorsOfClass "/Game/Blueprints/Entities/PlayerCharacter.PlayerCharacter_C"))
  (bind _output_get (LocalVariables|SetPotentialTargets _outactors))
  (LocalVariables|SetBestTarget 0)
  (for _array_element _output_get
    (Utilities|IsValid (LocalVariables|GetBestTarget)
      (:Is%20Valid
        (if (> (Class|HexFunctionLibrary|HDist (Default|GetActorHexPosition (LocalVariables|GetBestTarget)) _hexposition) (Class|HexFunctionLibrary|HDist (Default|GetActorHexPosition _array_element) _hexposition))
          (bind _asikillable (Utilities|Casting|CastToIKillable _array_element :!label _label)
            (:then
              (bind _dead (Default|IsDead _asikillable))
              (if (not _dead)
                (LocalVariables|SetBestTarget _array_element :!label _label_2)))
            (:CastFailed
              (goto _label_2)))))
      (:Is%20Not%20Valid
        (goto _label))))
  (return (LocalVariables|GetBestTarget)))

(fn Splat
  (bind _returnvalue (Transformation|GetActorLocation))
  (Utilities|SpawnActoronTile "/Game/Blueprints/Entities/PropSplat2.PropSplat2_C" (CallFunction|GetActorHexPosition))
  (if (Math|Random|RandomBool)
    (Audio|PlaySoundatLocation "/Game/Sound/Splat2.Splat2" _returnvalue)
    (else
      (Audio|PlaySoundatLocation "/Game/Sound/splat3.splat3" _returnvalue)))
  (Actor|DestroyActor))