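; Item is a base actor for world objects that a holder can pick up and drop.
; PickedUp stores the holder, marks the item held and hides the actor rather than destroying it.
; Drop teleports the item to the holder's location, clears the holder and held flag, and makes it visible again.
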(event Custom|Drop
  ;[1 1 1] Item Dropped
  (Transformation|SetActorLocation (Transformation|GetActorLocation (Variables|Default|Getholder)) false true)
  (Variables|Default|SetisHeld false)
  (Variables|Default|Setholder 0)
  (Rendering|SetActorHiddenInGame false))

(event Custom|Picked%20Up
  (params (Holder :type Player%20Character%20Object%20Reference))
  ;[1 1 1] Item Picked Up
  (Variables|Default|Setholder Holder)
  (Variables|Default|SetisHeld true)
  (Rendering|SetActorHiddenInGame true))

(event EventBeginPlay
  (|CallParentFunction))

(event Collision|EventActorBeginOverlap
  (params (OtherActor :type Actor%20Object%20Reference)))

(event EventTick
  (params (DeltaSeconds :type Float%20%28single-precision%29)))

(fn ConstructionScript
  (|CallParentFunction))