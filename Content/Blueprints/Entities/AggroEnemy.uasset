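; AggroEnemy is a turn-based hex-grid enemy that hunts the nearest living player character, growing more aggressive as victory points rise.
; At low aggression it moves to a random ring point near the target, then onward away from it.
; Otherwise it moves toward a random point in a radius that shrinks with aggression, with more move points.
; It kills targets sharing its hex when movement ends, and its mesh shows only when lit.
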(event TurnActivateDelegate(Turn)
  (bind _output_get (Variables|Default|SetCurrentTarget (CallFunction|ChooseTarget)))
  (Utilities|IsValid _output_get
    (:Is%20Valid
      (if (CallFunction|LowAggression)
        (CallFunction|StartMovetoPoints (Utilities|Array|MakeArray (CallFunction|EnemyTargetPoint (Default|GetActorHexPosition _output_get)) (CallFunction|MovefromLight (Default|GetActorHexPosition _output_get) (CallFunction|EnemyTargetPoint (Default|GetActorHexPosition _output_get)))) 10)
        (Class|TurnComponent|EndTurn (Variables|Default|GetTurn) :!label _label)
        (else
          (bind _canmove (CallFunction|StartMovetoPoint (CallFunction|EnemyTargetPoint (Default|GetActorHexPosition _output_get)) (CallFunction|CalculateAggression)))
          (if (not _canmove)
            (goto _label)))))
    (:Is%20Not%20Valid
      (goto _label))))

(event TurnEndDelegate(Turn))

(event EventOnMoveEnd
  (bind _currenttarget (Variables|Default|GetCurrentTarget))
  (Class|TurnComponent|EndTurn (Variables|Default|GetTurn))
  (bind _asikillable (Utilities|Casting|CastToIKillable _currenttarget))
  (if (Class|HexFunctionLibrary|EqualHexVectorHexVector (CallFunction|GetActorHexPosition) (Default|GetActorHexPosition _currenttarget))
    (Default|Kill _asikillable)))

(event EventOnLightUpdate
  (params (IsLit :type Boolean))
  (Development|SetHiddeninGame (Variables|Default|GetRootMesh) (not IsLit) false))

(event EventBeginPlay
  (|CallParentFunction))

(event EventTick
  (params (DeltaSeconds :type Float%20%28single-precision%29))
  (|CallParentFunction DeltaSeconds))

(fn ConstructionScript
  (|CallParentFunction))

(fn ChooseTarget
  (bind _hexposition (CallFunction|GetActorHexPosition))
  (bind _outactors (Actor|GetAllActorsOfClass "/Game/Blueprints/Entities/PlayerCharacter.PlayerCharacter_C"))
  (bind _output_get (LocalVariables|SetPotentialTargets _outactors))
  (LocalVariables|SetBestTarget 0)
  (for _array_element _output_get
    (Utilities|IsValid (LocalVariables|GetBestTarget)
      (:Is%20Valid
        (if (> (Class|HexFunctionLibrary|HDist (Default|GetActorHexPosition (LocalVariables|GetBestTarget)) _hexposition) (Class|HexFunctionLibrary|HDist (Default|GetActorHexPosition _array_element) _hexposition))
          (bind _asikillable (Utilities|Casting|CastToIKillable _array_element :!label _label)
            (:then
              (bind _dead (Default|IsDead _asikillable))
              (if (not _dead)
                (LocalVariables|SetBestTarget _array_element :!label _label_2)))
            (:CastFailed
              (goto _label_2)))))
      (:Is%20Not%20Valid
        (goto _label))))
  (return (LocalVariables|GetBestTarget)))

(fn EnemyTargetPoint
  (params (TargetPosition :type Hex%20Vector%20Structure))
  (bind _agressionlevel (CallFunction|CalculateAggression))
  (bind _returnvalue (- 3 _agressionlevel))
  (bind _returnvalue_2 (Class|HexFunctionLibrary|HexRing TargetPosition _returnvalue))
  (bind _returnvalue_3 (Class|HexFunctionLibrary|HexinRadius TargetPosition _returnvalue))
  (bind _returnvalue_4 (Utilities|Array|Length _returnvalue_3))
  (bind _returnvalue_5 (Utilities|Array|Length _returnvalue_2))
  (bind _returnvalue_6 (Math|Random|RandomInteger _returnvalue_5))
  (bind _returnvalue_7 (Math|Random|RandomInteger _returnvalue_4))
  (bind _output (Utilities|Array|Get(acopy) _returnvalue_3 _returnvalue_7))
  (bind _output_2 (Utilities|Array|Get(acopy) _returnvalue_2 _returnvalue_6))
  (if (CallFunction|LowAggression)
    (while (Variables|/Script/HexGameFramework.HexTileData|GetIsWall (Class|HexMap|GetDataatHex (Utilities|GetHexMap) _output_2))
      (bind _structout (Utilities|Struct|SetmembersinHexVector _output_2)))
    (return _structout)
    (else
      (while (Variables|/Script/HexGameFramework.HexTileData|GetIsWall (Class|HexMap|GetDataatHex (Utilities|GetHexMap) _output))
        (bind _structout_2 (Utilities|Struct|SetmembersinHexVector _output)))
      (return _structout_2))))

(fn CalculateAggression
  (return (+ (Default|GetVictoryPoints (Utilities|GetHexGameMode)) 1)))

(fn MovefromLight
  (params (TargetPosition :type Hex%20Vector%20Structure) (EnemyPosition :type Hex%20Vector%20Structure))
  (return (+ (- EnemyPosition TargetPosition) EnemyPosition)))

(fn LowAggression
  (return (<= (CallFunction|CalculateAggression) 1)))

(fn EnemyMultimove
  (params (TargetPosition :type Hex%20Vector%20Structure) (EnemyPosition :type Hex%20Vector%20Structure))
  (bind _movetotile (CallFunction|EnemyTargetPoint TargetPosition))
  (bind _moveto (CallFunction|MovefromLight TargetPosition EnemyPosition))
  (if (Class|HexMap|IsTileLitUp (Utilities|GetHexMap) _moveto)
    (bind _structout (Utilities|Struct|SetmembersinHexVector _moveto))
    (return (Utilities|Array|MakeArray _movetotile _structout))
    (else
      (while (Class|HexMap|IsTileLitUp (Utilities|GetHexMap))
        (bind _structout_2 (Utilities|Struct|SetmembersinHexVector)))
      (return (Utilities|Array|MakeArray _movetotile _structout_2)))))