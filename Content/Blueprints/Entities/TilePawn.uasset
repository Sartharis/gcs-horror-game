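; TilePawn is a pawn that travels across the hex map tile by tile along a path.
; StartMoveToPoint gets a path from the current hex map, stores the move points and opens a gate on Tick.
; Tick slides the pawn toward the next hex, then snaps to it, updates its hex position and spends a point.
; When the path or points run out, it fires the empty OnMoveEnd event and closes the gate.
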(event Custom|MoveAlongPath
  (params (Path :type Array%20of%20Hex%20Vector%20Structures))
  ;[1 1 1] Movement Events
  (Variables|Default|SetMovePath Path)
  (CallFunction|StartMovingAlongPath))

(event Custom|StartMovingAlongPath
  (bind _returnvalue (Transformation|GetActorLocation))
  (bind _hexgamemode (Utilities|GetHexGameMode))
  (bind _movepath (Variables|Default|GetMovePath))
  (bind _movepath_2 (Variables|Default|GetMovePath))
  (bind _output (Utilities|Array|Get(acopy) _movepath_2))
  (bind _currenthexmap (Variables|/Script/HexGameFramework.HexGameFrameworkGameModeBase|GetCurrentHexMap _hexgamemode))
  (bind _returnvalue_2 (Class|HexMap|HexVectortoPoint _currenthexmap _output))
  ;[1 1 1] Movement Events
  (if (> (Variables|Default|GetCurrentMovePoints) 0)
    (Utilities|FlowControl|Gate true) ; enters at Open
  ))

(event Custom|StopMovingAlongPath
  (bind _returnvalue (Transformation|GetActorLocation))
  (bind _hexgamemode (Utilities|GetHexGameMode))
  (bind _movepath (Variables|Default|GetMovePath))
  (bind _movepath_2 (Variables|Default|GetMovePath))
  (bind _output (Utilities|Array|Get(acopy) _movepath_2))
  (bind _currenthexmap (Variables|/Script/HexGameFramework.HexGameFrameworkGameModeBase|GetCurrentHexMap _hexgamemode))
  (bind _returnvalue_2 (Class|HexMap|HexVectortoPoint _currenthexmap _output))
  ;[1 1 1] Movement Events
  (Utilities|FlowControl|Gate true) ; enters at Close
)

(event Custom|OnMoveEnd
  ;[1 1 1] Movement Events
)

(event EventTick
  (params (DeltaSeconds :type Float%20%28single-precision%29))
  (bind _returnvalue (Transformation|GetActorLocation))
  (bind _hexgamemode (Utilities|GetHexGameMode))
  (bind _movepath (Variables|Default|GetMovePath))
  (bind _movepath_2 (Variables|Default|GetMovePath))
  (bind _movespeed (Variables|Default|GetMoveSpeed))
  (bind _returnvalue_2 (* _movespeed DeltaSeconds))
  (bind _output (Utilities|Array|Get(acopy) _movepath_2))
  (bind _currenthexmap (Variables|/Script/HexGameFramework.HexGameFrameworkGameModeBase|GetCurrentHexMap _hexgamemode))
  (bind _returnvalue_3 (Class|HexMap|HexVectortoPoint _currenthexmap _output))
  ;[1 1 1] Movement Events
  (|CallParentFunction DeltaSeconds)
  (Utilities|FlowControl|Gate true
    (:Exit
      (if (> (Utilities|Array|Length _movepath_2) 0)
        (if (<= (Math|Vector|VectorLengthSquared (- _returnvalue _returnvalue_3)) (Math|Float|Square _returnvalue_2))
          (Transformation|SetActorLocation _returnvalue_3 false false)
          (CallFunction|ChangeHexPosition _output)
          (bind _result (Math|Integer|DecrementInt (Variables|Default|GetCurrentMovePoints))
            (:%20%20
              (Utilities|Array|RemoveIndex _movepath)
              (if (or (== (Utilities|Array|Length _movepath) 0) (== _result 0))
                (CallFunction|OnMoveEnd)
                (CallFunction|StopMovingAlongPath))))
          (else
            (Transformation|AddActorLocalOffset (* (Math|Vector|GetUnitDirection(Vector) _returnvalue _returnvalue_3) _returnvalue_2) false false)))))))

(fn ConstructionScript
  (|CallParentFunction))

(fn StartMovetoPoint
  (params (TargetPoint :type Hex%20Vector%20Structure) (MovePoints :type Integer))
  (bind _hexposition (CallFunction|GetActorHexPosition))
  (bind _hexgamemode (Utilities|GetHexGameMode))
  (bind _currenthexmap (Variables|/Script/HexGameFramework.HexGameFrameworkGameModeBase|GetCurrentHexMap _hexgamemode))
  (bind _returnvalue (Class|HexMap|GetPathBetweenHexes _currenthexmap _hexposition TargetPoint))
  (if (Class|HexFunctionLibrary|EqualHexVectorHexVector _hexposition TargetPoint)
    (return false)
    (elif (> (Utilities|Array|Length _returnvalue) 0)
      (Variables|Default|SetCurrentMovePoints MovePoints)
      (CallFunction|MoveAlongPath _returnvalue)
      (return true)
      (else
        (return false)))))