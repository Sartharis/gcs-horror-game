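; Powered door entity for the horror game that can be activated, interacted with, broken and fixed.
; Activation and interaction share one toggle that flips actor blocking and instantly offsets the root mesh vertically by MoveDownZ, signed by BlockActors.
; Both are reported as available only while HorrorBaseGamemode has electricity on and the door is not broken.
; Break and Fix just set the Broken flag, and the door always reports it can be broken.
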(event EventBeginPlay
  (|CallParentFunction))

(event Collision|EventActorBeginOverlap
  (params (OtherActor :type Actor%20Object%20Reference)))

(event EventOnActivate
  (bind _blockactors (Variables|Default|GetBlockActors))
  (bind _movedownz (Variables|Default|GetMoveDownZ))
  (bind _rootmesh (Variables|Default|GetRootMesh))
  (Class|TileObject|SetBlocking (not _blockactors))
  (if _blockactors
    (Transformation|AddWorldOffset _rootmesh (Math|Vector|MakeVector 0.0 0.0 _movedownz) false false)
    (else
      (Transformation|AddWorldOffset _rootmesh (Math|Vector|MakeVector 0.0 0.0 (* _movedownz -1.0)) false false))))

(event EventOnInteraction
  (bind _blockactors (Variables|Default|GetBlockActors))
  (bind _movedownz (Variables|Default|GetMoveDownZ))
  (bind _rootmesh (Variables|Default|GetRootMesh))
  (Class|TileObject|SetBlocking (not _blockactors))
  (if _blockactors
    (Transformation|AddWorldOffset _rootmesh (Math|Vector|MakeVector 0.0 0.0 _movedownz) false false)
    (else
      (Transformation|AddWorldOffset _rootmesh (Math|Vector|MakeVector 0.0 0.0 (* _movedownz -1.0)) false false))))

(event EventTick
  (params (DeltaSeconds :type Float%20%28single-precision%29)))

(event EventFix
  (Variables|Default|SetBroken false))

(event EventBreak
  (Variables|Default|SetBroken true))

(fn ConstructionScript
  (|CallParentFunction))

(fn CanbeActivated
  (bind _ashorror_base_gamemode (Utilities|Casting|CastToHorrorBaseGamemode (Game|GetGameMode))
    (:then
      (return (and (Variables|/Game/Blueprints/HorrorBaseGamemode.HorrorBaseGamemode_C|Getelectricity_on _ashorror_base_gamemode) (not (Variables|Default|GetBroken)))))
    (:CastFailed
      (return false))))

(fn CanbeBroken
  (return true))

(fn CanbeInteractedwith
  (bind _ashorror_base_gamemode (Utilities|Casting|CastToHorrorBaseGamemode (Game|GetGameMode))
    (:then
      (return (and (Variables|/Game/Blueprints/HorrorBaseGamemode.HorrorBaseGamemode_C|Getelectricity_on _ashorror_base_gamemode) (not (Variables|Default|GetBroken)))))
    (:CastFailed
      (return false))))