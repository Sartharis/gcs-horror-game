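; Turn-based zombie enemy that hunts player characters on a hex grid and is visible only while lit.
; On its turn it picks the nearest player character not reported dead and starts a short move toward that character's hex, ending the turn if it cannot.
; When movement finishes it ends its turn, then kills the target through IKillable if both share a hex.
; Light updates toggle the root mesh's visibility.
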(event TurnActivateDelegate(Turn)
  (bind _output_get (Variables|Default|SetCurrentTarget (CallFunction|ChooseTarget)))
  (Utilities|IsValid _output_get
    (:Is%20Valid
      (bind _canmove (CallFunction|StartMovetoPoint (Default|GetActorHexPosition _output_get) 2))
      (if (not _canmove)
        (Class|TurnComponent|EndTurn (Variables|Default|GetTurn) :!label _label)))
    (:Is%20Not%20Valid
      (goto _label))))

(event TurnEndDelegate(Turn))

(event EventOnMoveEnd
  (bind _currenttarget (Variables|Default|GetCurrentTarget))
  (Class|TurnComponent|EndTurn (Variables|Default|GetTurn))
  (bind _asikillable (Utilities|Casting|CastToIKillable _currenttarget))
  (if (Class|HexFunctionLibrary|EqualHexVectorHexVector (CallFunction|GetActorHexPosition) (Default|GetActorHexPosition _currenttarget))
    (Default|Kill _asikillable)))

(event EventOnLightUpdate
  (params (IsLit :type Boolean))
  (Development|SetHiddeninGame (Variables|Default|GetRootMesh) (not IsLit) false))

(event EventBeginPlay
  (|CallParentFunction))

(event EventTick
  (params (DeltaSeconds :type Float%20%28single-precision%29))
  (|CallParentFunction DeltaSeconds))

(fn ConstructionScript
  (|CallParentFunction))

(fn ChooseTarget
  (bind _hexposition (CallFunction|GetActorHexPosition))
  (bind _outactors (Actor|GetAllActorsOfClass "/Game/Blueprints/Entities/PlayerCharacter.PlayerCharacter_C"))
  (bind _output_get (LocalVariables|SetPotentialTargets _outactors))
  (LocalVariables|SetBestTarget 0)
  (for _array_element _output_get
    (Utilities|IsValid (LocalVariables|GetBestTarget)
      (:Is%20Valid
        (if (> (Class|HexFunctionLibrary|HDist (Default|GetActorHexPosition (LocalVariables|GetBestTarget)) _hexposition) (Class|HexFunctionLibrary|HDist (Default|GetActorHexPosition _array_element) _hexposition))
          (bind _asikillable (Utilities|Casting|CastToIKillable _array_element :!label _label)
            (:then
              (bind _dead (Default|IsDead _asikillable))
              (if (not _dead)
                (LocalVariables|SetBestTarget _array_element :!label _label_2)))
            (:CastFailed
              (goto _label_2)))))
      (:Is%20Not%20Valid
        (goto _label))))
  (return (LocalVariables|GetBestTarget)))