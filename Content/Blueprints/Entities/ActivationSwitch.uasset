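; ActivationSwitch is an interactable switch that activates a list of linked actors.
; Interaction flips its On state, then calls OnActivate on each ActorsToActivate entry whose IActivateable CanBeActivated check passes, regardless of the new state.
; Entries lacking the interface print a warning.
; CanBeInteractedWith blocks use when the switch is Broken, or already On and not Toggleable.
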(event EventOnInteraction
  (Variables|Default|SetOn (not (Variables|Default|GetOn)))
  (for _array_element (Variables|Default|GetActorsToActivate)
    (bind _asiactivateable (Utilities|Casting|CastToIActivateable _array_element)
      (:then
        (bind _canbeactivated (Default|CanbeActivated _asiactivateable))
        (if _canbeactivated
          (Default|OnActivate _asiactivateable)))
      (:CastFailed
        (Development|PrintString (Utilities|String|Append (Utilities|String|ToString(Object) _array_element) " was activated but is not IActivatable!"))))))

(fn ConstructionScript
  (|CallParentFunction))

(fn CanbeInteractedwith
  (return (and (or (Variables|Default|GetToggleable) (not (Variables|Default|GetOn))) (not (Variables|Default|GetBroken)))))