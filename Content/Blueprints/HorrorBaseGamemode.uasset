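; Game mode for a turn-based horror game that runs the main HUD, item-collection win, all-players-dead loss and electrical power system.
; Switched lights add to a power load; reaching the limit or calling ShutDownElectricity kills all ceiling lights and toggles non-blocking doors.
; A TurnManager round-start binding restores power two rounds later, relighting only lights not wired to switches and re-toggling recorded doors.
; The HUD announces monster turns, power load and game outcomes.
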(event Custom|onPlayerDeath
  (Variables|Default|Setdead_all true)
  (bind _outactors (Actor|GetAllActorsOfClass "/Game/Blueprints/Entities/PlayerCharacter.PlayerCharacter_C"))
  (for _array_element _outactors
    (if (not (stale _dead))
      (Variables|Default|Setdead_all false)))
  (if (Variables|Default|Getdead_all)
    (Default|DisplayText (Variables|Default|GetMainUI) "You Died" 1e+01)))

(event Custom|OnVictoryDrop
  (Variables|Default|Setitem_pickup (+ (Variables|Default|Getitem_pickup) -1)))

(event Custom|OnDrop
  (Math|Integer|DecrementInt (Variables|Default|Getitem_pickup)))

(event Custom|turnElecOn
  (params (CurrentRound :type Integer))
  (if (and (>= CurrentRound (+ (Variables|Default|Getelec_off_round) 2)) (not (Variables|Default|Getelectricity_on)))
    (Variables|Default|Setelectricity_on true)
    (Variables|Default|Setlight_current 0)
    (for _array_element (Variables|Default|Getunactivatable_lights)
      (Class|HexLightComponent|ToggleLight (Variables|/Game/Blueprints/Entities/LightItems/CeilingLight.CeilingLight_C|GetHexLight _array_element) true))
    (for _array_element_2 (Variables|Default|Getdoors_open)
      (Default|OnActivate _array_element_2))))

(event Custom|onLightSwitched
  (params (On :type Boolean))
  (bind _mainui (Variables|Default|GetMainUI))
  (bind _light_max (Variables|Default|Getlight_max))
  (bind _output_get (Variables|Default|Setlight_current (+ (stale _output_get) (Math|Float|Round (* 2 (- (Math|Conversions|ToFloat(Boolean) On) 0.5))))))
  (if (>= (Variables|Default|Getlight_current) _light_max)
    (Default|DisplayText _mainui "Power Overload!" 1.0)
    (bind _outactors (Actor|GetAllActorsOfClass "/Game/Blueprints/Entities/LightItems/CeilingLight.CeilingLight_C"))
    (for _array_element _outactors
      (bind _asceiling_light (Utilities|Casting|CastToCeilingLight _array_element))
      (Class|HexLightComponent|ToggleLight (Variables|/Game/Blueprints/Entities/LightItems/CeilingLight.CeilingLight_C|GetHexLight _asceiling_light) false))
    (Variables|Default|Setelectricity_on false)
    (Variables|Default|Setelec_off_round (Class|TurnManager|GetCurrentRound (Class|HexGameFrameworkGameModeBase|GetTurnManager)))
    (Audio|PlaySound2D "/Game/Descending.Descending")
    (EventDispatchers|BindEventtoRoundStart (Class|HexGameFrameworkGameModeBase|GetTurnManager) (delegate Custom|turnElecOn))
    (bind _outactors_2 (Actor|GetAllActorsOfClass "/Game/Blueprints/Entities/Door.Door_C"))
    (for _array_element_2 _outactors_2
      (if (not (Variables|/Script/HexGameFramework.TileObject|GetBlockActors _array_element_2))
        (Default|OnActivate _array_element_2)
        (Utilities|Array|Insert (Variables|Default|Getdoors_open) _array_element_2)))
    (else
      (Default|DisplayText _mainui (Utilities|String|Append (Utilities|String|ToString(Integer) (Math|Float|Round (* (/ (Math|Conversions|ToFloat(Integer) (Variables|Default|Getlight_current)) (Math|Conversions|ToFloat(Integer) (- _light_max 1))) 1e+02))) "%" " Power") 1.0))))

(event Custom|TurnStart_Event_0
  (params (TurnCategory :type ETurnCategory%20Enum :default "TC_PLAYER"))
  (bind _mainui (Variables|Default|GetMainUI))
  (if (Utilities|Enum|Equal(Enum) TurnCategory "TC_ENEMY")
    (Default|DisplayText _mainui "MONSTER TURN" 1e+02)
    (else
      (Default|HideText _mainui))))

(event Custom|OnVictoryPickup
  (bind _output_get (Variables|Default|Setitem_pickup (+ (Variables|Default|Getitem_pickup) 1)))
  (bind _output_get_2 (Variables|Default|Setitem_all (== _output_get (Variables|Default|Getitem_max))))
  (if _output_get_2
    (Default|DisplayText (Variables|Default|GetMainUI) "You Win" 1e+01)))

(event Custom|ShutDownElectricity
  (bind _outactors (Actor|GetAllActorsOfClass "/Game/Blueprints/Entities/LightItems/CeilingLight.CeilingLight_C"))
  (for _array_element _outactors
    (bind _asceiling_light (Utilities|Casting|CastToCeilingLight _array_element))
    (Class|HexLightComponent|ToggleLight (Variables|/Game/Blueprints/Entities/LightItems/CeilingLight.CeilingLight_C|GetHexLight _asceiling_light) false))
  (Variables|Default|Setelectricity_on false)
  (Variables|Default|Setelec_off_round (Class|TurnManager|GetCurrentRound (Class|HexGameFrameworkGameModeBase|GetTurnManager)))
  (Audio|PlaySound2D "/Game/Descending.Descending")
  (EventDispatchers|BindEventtoRoundStart (Class|HexGameFrameworkGameModeBase|GetTurnManager) (delegate Custom|turnElecOn))
  (bind _outactors_2 (Actor|GetAllActorsOfClass "/Game/Blueprints/Entities/Door.Door_C"))
  (for _array_element_2 _outactors_2
    (if (not (Variables|/Script/HexGameFramework.TileObject|GetBlockActors _array_element_2))
      (Default|OnActivate _array_element_2)
      (Utilities|Array|Insert (Variables|Default|Getdoors_open) _array_element_2))))

(event EventTick
  (params (DeltaSeconds :type Float%20%28single-precision%29))
  (EventDispatchers|AssignTurnStart (Variables|Default|GetTurnManager) (delegate Custom|TurnStart_Event_0)))

(event EventBeginPlay
  (|CallParentFunction)
  (Variables|Default|Setlight_current 0)
  (bind _outactors (Actor|GetAllActorsOfClass "/Game/Blueprints/Entities/Item.Item_C"))
  (Variables|Default|Setitem_max (Utilities|Array|Length _outactors))
  (Variables|Default|Setlight_max 3)
  (bind _outactors_2 (Actor|GetAllActorsOfClass "/Game/Blueprints/Entities/ActivationSwitch.ActivationSwitch_C"))
  (for _array_element _outactors_2
    (for _array_element_2 (Variables|/Game/Blueprints/Entities/ActivationSwitch.ActivationSwitch_C|GetActorsToActivate _array_element)
      (bind _asceiling_light (Utilities|Casting|CastToCeilingLight _array_element_2))
      (Utilities|Array|Insert (Variables|Default|Getactivatable_lights) _asceiling_light)))
  (bind _outactors_3 (Actor|GetAllActorsOfClass "/Game/Blueprints/Entities/LightItems/CeilingLight.CeilingLight_C"))
  (for _array_element_3 _outactors_3
    (if (not (Utilities|Array|ContainsItem (Variables|Default|Getactivatable_lights) _array_element_3))
      (Utilities|Array|Add (Variables|Default|Getunactivatable_lights) _array_element_3)))
  (bind _returnvalue (UserInterface|CreateWidget "/Game/Blueprints/MainUI.MainUI_C"))
  (bind _output_get (Variables|Default|SetMainUI _returnvalue))
  (UserInterface|Viewport|AddtoViewport _output_get 0))

(fn ConstructionScript
  (|CallParentFunction))

(fn SpawnDefaultPawnfor
  (params (NewPlayer :type Controller%20Object%20Reference) (StartSpot :type Actor%20Object%20Reference))
  (return 0))

(fn GetVictoryPoints
  (return (Variables|Default|Getitem_pickup)))