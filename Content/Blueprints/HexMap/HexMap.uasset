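; HexMap is the hex-grid map actor that registers itself with the hex game mode and draws fog over unlit tiles.
; After BeginPlay it refreshes every tile, placing FogMeshes instances on dark non-wall hexes, tracked per hex in ShadowIndices.
; Lit or wall hexes move their instance below ground into a reuse pool rather than removing it.
; UpdateMeshShadows also passes lit state to TileActors on each changed tile.
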(event EventBeginPlay
  (Variables|/Script/HexGameFramework.HexGameFrameworkGameModeBase|SetCurrentHexMap (Utilities|GetHexGameMode) self)
  (Utilities|FlowControl|Delay 0.0)
  (Class|HexMap|UpdateAllMeshShadows))

(event EventUpdateMeshShadows
  (params (ChangedTiles :type Array%20of%20Hex%20Vector%20Structures))
  (bind _shadowindices (Variables|Default|GetShadowIndices))
  (bind _fogmeshes (Variables|Default|GetFogMeshes))
  (bind _unusedshadowindices (Variables|Default|GetUnusedShadowIndices))
  (bind _shadowindices_2 (Variables|Default|GetShadowIndices))
  (bind _output (Utilities|Array|Get(acopy) _unusedshadowindices))
  (for _array_element ChangedTiles
    (if (or (Variables|/Script/HexGameFramework.HexTileData|GetIsWall (Class|HexMap|GetDataatHex _array_element)) (Class|HexMap|IsTileLitUp _array_element))
      (if (.ReturnValue (Utilities|Map|Find _shadowindices_2 _array_element))
        (Utilities|Array|Add (Variables|Default|GetUnusedShadowIndices) (.Value (Utilities|Map|Find _shadowindices_2 _array_element)))
        (Components|InstancedStaticMesh|UpdateInstanceTransform (Variables|Default|GetFogMeshes) (.Value (Utilities|Map|Find _shadowindices_2 _array_element)) (Math|Transform|MakeTransform "0, 0,-500.000000" "0, 0, 0" "1,1,1") true true false)
        (Utilities|Map|Remove _shadowindices_2 _array_element))
      (elif (not (.ReturnValue (Utilities|Map|Find (Variables|Default|GetShadowIndices) _array_element)))
        (if (> (Utilities|Array|Length _unusedshadowindices) 0)
          (Components|InstancedStaticMesh|UpdateInstanceTransform _fogmeshes _output (Math|Transform|MakeTransform (Class|HexMap|HexVectortoPoint _array_element) "0, 0, 0" "1,1,1") true true false)
          (Utilities|Map|Add _shadowindices _array_element _output)
          (Utilities|Array|RemoveIndex _unusedshadowindices)
          (else
            (bind _returnvalue (Class|InstancedStaticMeshComponent|AddInstanceWorldSpace _fogmeshes (Math|Transform|MakeTransform (Class|HexMap|HexVectortoPoint _array_element) "0, 0, 0" "1,1,1")))
            (Utilities|Map|Add _shadowindices _array_element _returnvalue))))))
  (for _array_element_2 ChangedTiles
    (bind _result (Utilities|Set|ToArray (Variables|/Script/HexGameFramework.HexTileData|GetActorsOnTile (Class|HexMap|GetDataatHex _array_element_2))))
    (for _array_element_3 _result
      (bind _astile_actor (Utilities|Casting|CastToTileActor _array_element_3))
      (Default|OnLightUpdate _astile_actor (Class|HexMap|IsTileLitUp _array_element_2)))))

(event EventNotifyTileActorsOfLightChange)

(event EventUpdateAllMeshShadows
  (Class|HexMap|UpdateMeshShadows (Class|HexMap|GetAllTilesonMap)))

(fn ConstructionScript)