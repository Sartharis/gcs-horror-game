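; TileRemover is a placeable actor that deletes tiles from a HexMap within a hex radius when RemoveTiles is enabled.
; Its construction script finds the overlapping HexMap through SnapCollision and snaps RootMesh to the nearest hex.
; Surrounding hexes are removed with mesh updates deferred, then the center hex is removed with an update and all instanced meshes refresh.
; SnapCollision is disabled at BeginPlay because only construction uses it.
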(event EventBeginPlay
  (Collision|SetCollisionEnabled (Variables|Default|GetSnapCollision) "NoCollision") ; We turn off the collsion, since we only use it in the construction script
)

(fn ConstructionScript
  ;[1 1 1] Tile snapping and initial position setting
  (bind _outactors (Collision|ComponentOverlapActors (Variables|Default|GetSnapCollision) (Transformation|GetActorTransform) (Utilities|Array|MakeArray "ObjectTypeQuery2") "/Game/Blueprints/HexMap/HexMap.HexMap_C"))
  (Transformation|SetWorldLocation (Variables|Default|GetRootMesh) (Class|HexMap|HexVectortoPoint (.AsHex%20Map (Utilities|Casting|CastToHexMap (Utilities|Array|Get(acopy) _outactors))) (Class|HexMap|PointtoHexVector (.AsHex%20Map (Utilities|Casting|CastToHexMap (Utilities|Array|Get(acopy) _outactors))) (Transformation|GetWorldLocation (Variables|Default|GetDefaultSceneRoot)))) false false)
  (if (Variables|Default|GetRemoveTiles)
    (for _array_element (Class|HexFunctionLibrary|HexinRadius (Class|HexMap|PointtoHexVector (.AsHex%20Map (Utilities|Casting|CastToHexMap (Utilities|Array|Get(acopy) _outactors))) (Transformation|GetWorldLocation (Variables|Default|GetDefaultSceneRoot))) (Variables|Default|GetRadius))
      (if (not (Class|HexFunctionLibrary|EqualHexVectorHexVector _array_element (Class|HexMap|PointtoHexVector (.AsHex%20Map (Utilities|Casting|CastToHexMap (Utilities|Array|Get(acopy) _outactors))) (Transformation|GetWorldLocation (Variables|Default|GetDefaultSceneRoot)))))
        (Class|HexMap|RemoveHex (.AsHex%20Map (Utilities|Casting|CastToHexMap (Utilities|Array|Get(acopy) _outactors))) _array_element false)))
    (Class|HexMap|RemoveHex (.AsHex%20Map (Utilities|Casting|CastToHexMap (Utilities|Array|Get(acopy) _outactors))) (Class|HexMap|PointtoHexVector (.AsHex%20Map (Utilities|Casting|CastToHexMap (Utilities|Array|Get(acopy) _outactors))) (Transformation|GetWorldLocation (Variables|Default|GetDefaultSceneRoot))) true)
    (Class|HexMap|UpdateAllInstancedMeshes (.AsHex%20Map (Utilities|Casting|CastToHexMap (Utilities|Array|Get(acopy) _outactors))))))