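; TilePainter is an editor-time brush actor that paints a chosen tile type onto a HexMap as it is constructed.
; Its construction script finds the HexMap through an overlap on SnapCollision and snaps RootMesh to the hex under the actor.
; It changes differing hexes within Radius, batching their instanced mesh update, and handles the centre hex separately.
; SnapCollision serves only construction, so BeginPlay disables it.
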(event EventBeginPlay
  (Collision|SetCollisionEnabled (Variables|Default|GetSnapCollision) "NoCollision") ; We turn off the collsion, since we only use it in the construction script
)

(fn ConstructionScript
  (bind _radius (Variables|Default|GetRadius))
  (bind _tiletopaint (Variables|Default|GetTileToPaint))
  (bind _tiletopaint_2 (Variables|Default|GetTileToPaint))
  ;[1 1 1] Tile snapping and initial position setting
  (bind _outactors (Collision|ComponentOverlapActors (Variables|Default|GetSnapCollision) (Transformation|GetActorTransform) (Utilities|Array|MakeArray "ObjectTypeQuery2") "/Game/Blueprints/HexMap/HexMap.HexMap_C"))
  (Transformation|SetWorldLocation (Variables|Default|GetRootMesh) (Class|HexMap|HexVectortoPoint (.AsHex%20Map (Utilities|Casting|CastToHexMap (Utilities|Array|Get(acopy) _outactors))) (Class|HexMap|PointtoHexVector (.AsHex%20Map (Utilities|Casting|CastToHexMap (Utilities|Array|Get(acopy) _outactors))) (Transformation|GetWorldLocation (Variables|Default|GetDefaultSceneRoot)))) false false)
  (if (> _radius 1)
    (for _array_element (Class|HexFunctionLibrary|HexinRadius (Class|HexMap|PointtoHexVector (.AsHex%20Map (Utilities|Casting|CastToHexMap (Utilities|Array|Get(acopy) _outactors))) (Transformation|GetWorldLocation (Variables|Default|GetDefaultSceneRoot))) _radius)
      (if (Math|Boolean|ANDBoolean (!= _tiletopaint (Variables|/Script/HexGameFramework.HexTileData|GetHexTileType (Class|HexMap|GetDataatHex (.AsHex%20Map (Utilities|Casting|CastToHexMap (Utilities|Array|Get(acopy) _outactors))) _array_element))) (!= _tiletopaint 0) (not (Class|HexFunctionLibrary|EqualHexVectorHexVector _array_element (Class|HexMap|PointtoHexVector (.AsHex%20Map (Utilities|Casting|CastToHexMap (Utilities|Array|Get(acopy) _outactors))) (Transformation|GetWorldLocation (Variables|Default|GetDefaultSceneRoot))))))
        (Class|HexMap|AddorChangeHex (.AsHex%20Map (Utilities|Casting|CastToHexMap (Utilities|Array|Get(acopy) _outactors))) _array_element _tiletopaint false)))
    (Class|HexMap|UpdateAllInstancedMeshes (.AsHex%20Map (Utilities|Casting|CastToHexMap (Utilities|Array|Get(acopy) _outactors)))))
  (if (and (!= _tiletopaint_2 (Variables|/Script/HexGameFramework.HexTileData|GetHexTileType (Class|HexMap|GetDataatHex (.AsHex%20Map (Utilities|Casting|CastToHexMap (Utilities|Array|Get(acopy) _outactors))) (Class|HexMap|PointtoHexVector (.AsHex%20Map (Utilities|Casting|CastToHexMap (Utilities|Array|Get(acopy) _outactors))) (Transformation|GetWorldLocation (Variables|Default|GetDefaultSceneRoot)))))) (!= _tiletopaint_2 0))
    (Class|HexMap|AddorChangeHex (.AsHex%20Map (Utilities|Casting|CastToHexMap (Utilities|Array|Get(acopy) _outactors))) (Class|HexMap|PointtoHexVector (.AsHex%20Map (Utilities|Casting|CastToHexMap (Utilities|Array|Get(acopy) _outactors))) (Transformation|GetWorldLocation (Variables|Default|GetDefaultSceneRoot))) _tiletopaint_2 true)))