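; ISelectable is a Blueprint interface for selectable objects that take orders on a turn-based hex grid.
; It declares selection callbacks and queries for selectability, selection location, movement points and actors to ignore.
; Action and ability orders take a target hex and report acceptance, with action orders also flagging a position change, alongside ability-select and end-turn hooks.
; The graphs hold no logic, only empty or default returns.
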(fn OnSelected)

(fn OnUnselected)

(fn CanbeSelected
  (return false))

(fn OnEndTurnOrder)

(fn OnAbilityOrder
  (params (TargetHex :type Hex%20Vector%20Structure))
  (return false))

(fn OnAbilitySelect)

(fn GetSelectionLocation
  (return "0, 0, 0"))

(fn GetMovementPoints
  (return 0))

(fn OnActionOrder
  (params (TargetHex :type Hex%20Vector%20Structure))
  (return false false ""))

(fn GetActorstoIgnore
  (return 0))