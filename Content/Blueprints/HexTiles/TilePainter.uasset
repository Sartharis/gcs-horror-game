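; TilePainter is an editor placement tool that paints hex tiles onto a HexMap from its construction script.
; It finds the overlapping HexMap through SnapCollision, converts its root location to a hex coordinate and snaps RootMesh to that hex's point.
; When TileToPaint passes its check, it adds or changes that hex on the map and requests a mesh update.
; BeginPlay disables SnapCollision, which only serves construction.
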(event EventBeginPlay
  (Collision|SetCollisionEnabled (Variables|Default|GetSnapCollision) "NoCollision") ; We turn off the collsion, since we only use it in the construction script
)

(fn ConstructionScript
  (bind _tiletopaint (Variables|Default|GetTileToPaint))
  ;[1 1 1] Tile snapping and initial position setting
  (bind _outactors (Collision|ComponentOverlapActors (Variables|Default|GetSnapCollision) (Transformation|GetActorTransform) (Utilities|Array|MakeArray "ObjectTypeQuery2") "/Game/Blueprints/HexMap.HexMap_C"))
  (Transformation|SetWorldLocation (Variables|Default|GetRootMesh) (Class|HexMap|HexVectortoPoint (.AsHex%20Map (Utilities|Casting|CastToHexMap (Utilities|Array|Get(acopy) _outactors))) (Class|HexMap|PointtoHexVector (.AsHex%20Map (Utilities|Casting|CastToHexMap (Utilities|Array|Get(acopy) _outactors))) (Transformation|GetWorldLocation (Variables|Default|GetDefaultSceneRoot)))) false false)
  (if (!= _tiletopaint 0)
    (Class|HexMap|AddorChangeHex (.AsHex%20Map (Utilities|Casting|CastToHexMap (Utilities|Array|Get(acopy) _outactors))) (Class|HexMap|PointtoHexVector (.AsHex%20Map (Utilities|Casting|CastToHexMap (Utilities|Array|Get(acopy) _outactors))) (Transformation|GetWorldLocation (Variables|Default|GetDefaultSceneRoot))) _tiletopaint true)))