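; Player camera pawn and input controller for a hex-tile map, which registers itself with the hex game mode.
; Each tick a selector snaps to the hex under the mouse, found by intersecting the deprojected cursor ray with the map plane.
; Left click selects the first selectable actor on that tile via ISelectable, and right click sends it a move order.
; Axis inputs pan the spring-arm camera, and a helper draws hex paths as debug arrows.
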(event Custom|UnselectAll
  (Default|OnUnselected (Variables|Default|GetSelectedActor))
  (Variables|Default|SetSelectedActor 0))

(event EventBeginPlay
  (bind _returnvalue (Game|GetPlayerController 0))
  (|CallParentFunction)
  (Game|Player|SetViewTargetwithBlend _returnvalue self 0.0 "VTBlend_Linear" 0.0 false)
  (Development|SetHiddeninGame (Variables|Default|GetRootMesh) true false)
  (Variables|/Script/Engine.PlayerController|SetbShowMouseCursor _returnvalue true)
  (Rendering|SetVisibility (Variables|Default|GetSelector) true true)
  (Variables|/Script/HexGameFramework.HexGameFrameworkGameModeBase|SetPlayerController (Utilities|GetHexGameMode) self))

(event EventTick
  (params (DeltaSeconds :type Float%20%28single-precision%29))
  (bind (_currenthexmap _hexcoordinate) (CallFunction|GetHexCoordinateUnderMouse))
  (Transformation|SetWorldLocation (Variables|Default|GetSelector) (+ (Class|HexMap|HexVectortoPoint _currenthexmap _hexcoordinate) (Math|Vector|MakeVector 0.0 0.0 (.SelectionDrawHeight (Utilities|GetClassDefaults (Variables|/Script/HexGameFramework.HexTileData|GetHexTileType (Class|HexMap|GetDataatHex _currenthexmap _hexcoordinate)))))) false false))

(event Input|AxisEvents|InputAxisMoveScreenHorizontal
  (params (AxisValue :type Float%20%28single-precision%29))
  (Transformation|AddWorldOffset (Variables|Default|GetSpringArm) (Math|Vector|MakeVector 0.0 (* AxisValue (Variables|Default|GetCameraMoveSpeed)) 0.0) false false))

(event Input|AxisEvents|InputAxisMoveScreenVertical
  (params (AxisValue :type Float%20%28single-precision%29))
  (Transformation|AddWorldOffset (Variables|Default|GetSpringArm) (Math|Vector|MakeVector (* AxisValue (Variables|Default|GetCameraMoveSpeed)) 0.0 0.0) false false))

(event Input|MouseEvents|LeftMouseButton
  (params (Key :type Key%20Structure :default "AnyKey"))
  (bind (_currenthexmap _hexcoordinate) (CallFunction|GetHexCoordinateUnderMouse))
  (bind _returnvalue (Class|HexMap|GetDataatHex _currenthexmap _hexcoordinate))
  (bind _actorsontile (Variables|/Script/HexGameFramework.HexTileData|GetActorsOnTile _returnvalue))
  (:Pressed
    (if (> (Utilities|Set|Length _actorsontile) 0)
      (bind _result (Utilities|Set|ToArray _actorsontile))
      (bind _array_element (Utilities|Array|ForEachLoopwithBreak _result :!label _label)
        (:LoopBody
          (bind _asiselectable (Utilities|Casting|CastToISelectable _array_element))
          (bind _canbeselected (Default|CanbeSelected _asiselectable))
          (if _canbeselected
            (Default|OnUnselected (Variables|Default|GetSelectedActor))
            (bind _output_get (Variables|Default|SetSelectedActor _asiselectable))
            (Default|OnSelected _output_get)
            (goto _label Break))))
      (else
        (Default|OnUnselected (Variables|Default|GetSelectedActor))
        (Variables|Default|SetSelectedActor 0)))))

(event Input|MouseEvents|RightMouseButton
  (params (Key :type Key%20Structure :default "AnyKey"))
  (:Pressed
    (Default|OnMoveOrder (Variables|Default|GetSelectedActor) (.HexCoordinate (CallFunction|GetHexCoordinateUnderMouse)))))

(fn ConstructionScript
  (|CallParentFunction)
  (Transformation|SetWorldLocation (Variables|Default|GetSpringArm) (Transformation|GetWorldLocation (Variables|Default|GetRootMesh)) false false))

(fn GetHexCoordinateUnderMouse
  (bind _returnvalue (Game|GetPlayerController 0))
  (bind _hexgamemode (Utilities|GetHexGameMode))
  (bind (_worldlocation _worlddirection) (Game|Player|ConvertMouseLocationToWorldSpace _returnvalue))
  (bind _currenthexmap (Variables|/Script/HexGameFramework.HexGameFrameworkGameModeBase|GetCurrentHexMap _hexgamemode))
  (return _currenthexmap (Class|HexMap|PointtoHexVector _currenthexmap (.Intersection (Class|KismetMathLibrary|LinePlaneIntersectionOriginNormal _worldlocation (+ _worldlocation (* _worlddirection 8e+03)) (Transformation|GetActorLocation _currenthexmap) "0,0.000000,1.000000")))))

(fn DrawDebugPath
  (params (Start :type Hex%20Vector%20Structure) (End :type Hex%20Vector%20Structure))
  (bind _hexgamemode (Utilities|GetHexGameMode))
  (bind _currenthexmap (Variables|/Script/HexGameFramework.HexGameFrameworkGameModeBase|GetCurrentHexMap _hexgamemode))
  (bind _returnvalue (Class|HexMap|GetPathBetweenHexes _currenthexmap Start End))
  (bind _returnvalue_2 (Utilities|Array|Length _returnvalue))
  (for _index (range 0 (- _returnvalue_2 2))
    (Rendering|Debug|DrawDebugArrow :LineStart (+ (Class|HexMap|HexVectortoPoint _currenthexmap (Utilities|Array|Get(acopy) _returnvalue _index)) "0, 0,20.000000") :LineEnd (+ (Class|HexMap|HexVectortoPoint _currenthexmap (Utilities|Array|Get(acopy) _returnvalue (+ _index 1))) "0, 0,20.000000") :ArrowSize 1e+02 :Duration 0.0 :Thickness 1e+01))
  (if (> _returnvalue_2 0)
    (Rendering|Debug|DrawDebugArrow :LineStart (+ (Class|HexMap|HexVectortoPoint _currenthexmap Start) "0, 0,20.000000") :LineEnd (+ (Class|HexMap|HexVectortoPoint _currenthexmap (Utilities|Array|Get(acopy) _returnvalue)) "0, 0,20.000000") :ArrowSize 1e+02 :Thickness 1e+01)))