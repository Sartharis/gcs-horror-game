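; TilePawn is a pawn that moves along a path of hex tiles on the game mode's current hex map.
; MoveAlongPath stores the path and opens a Tick gate, which StopMovingAlongPath closes.
; Each tick it applies a MoveSpeed local offset toward the next hex, not scaled by DeltaSeconds, snapping when within range.
; Each arrival calls ChangePosition and pops that hex, firing the empty OnMoveEnd hook after the last.
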(event Custom|MoveAlongPath
  (params (Path :type Array%20of%20Hex%20Vector%20Structures))
  (Variables|Default|SetMovePath Path)
  (CallFunction|StartMovingAlongPath))

(event Custom|StartMovingAlongPath
  (bind _returnvalue (Transformation|GetActorLocation))
  (bind _hexgamemode (Utilities|GetHexGameMode))
  (bind _movepath (Variables|Default|GetMovePath))
  (bind _movepath_2 (Variables|Default|GetMovePath))
  (bind _item (Utilities|Array|Get(acopy) _movepath_2))
  (bind _currenthexmap (Variables|/Script/HexGameFramework.HexGameFrameworkGameModeBase|GetCurrentHexMap _hexgamemode))
  (bind _returnvalue_2 (Class|HexMap|HexVectortoPoint _currenthexmap _item))
  (Utilities|FlowControl|Gate true) ; enters at Open
)

(event Custom|StopMovingAlongPath
  (bind _returnvalue (Transformation|GetActorLocation))
  (bind _hexgamemode (Utilities|GetHexGameMode))
  (bind _movepath (Variables|Default|GetMovePath))
  (bind _movepath_2 (Variables|Default|GetMovePath))
  (bind _item (Utilities|Array|Get(acopy) _movepath_2))
  (bind _currenthexmap (Variables|/Script/HexGameFramework.HexGameFrameworkGameModeBase|GetCurrentHexMap _hexgamemode))
  (bind _returnvalue_2 (Class|HexMap|HexVectortoPoint _currenthexmap _item))
  (Utilities|FlowControl|Gate true) ; enters at Close
)

(event Custom|OnMoveEnd)

(event EventTick
  (params (DeltaSeconds :type Float%20%28single-precision%29))
  (bind _returnvalue (Transformation|GetActorLocation))
  (bind _hexgamemode (Utilities|GetHexGameMode))
  (bind _movepath (Variables|Default|GetMovePath))
  (bind _movepath_2 (Variables|Default|GetMovePath))
  (bind _item (Utilities|Array|Get(acopy) _movepath_2))
  (bind _currenthexmap (Variables|/Script/HexGameFramework.HexGameFrameworkGameModeBase|GetCurrentHexMap _hexgamemode))
  (bind _returnvalue_2 (Class|HexMap|HexVectortoPoint _currenthexmap _item))
  (|CallParentFunction DeltaSeconds)
  (Utilities|FlowControl|Gate true
    (:Exit
      (if (> (Utilities|Array|Length _movepath_2) 0)
        (if (<= (Math|Vector|VectorLengthSquared (- _returnvalue _returnvalue_2)) (Math|Float|Square (Variables|Default|GetMoveSpeed)))
          (Transformation|SetActorLocation _returnvalue_2 false false)
          (CallFunction|ChangePosition _item)
          (Utilities|Array|RemoveIndex _movepath)
          (if (== (Utilities|Array|Length _movepath) 0)
            (CallFunction|OnMoveEnd))
          (else
            (Transformation|AddActorLocalOffset (* (Math|Vector|GetUnitDirection(Vector) _returnvalue _returnvalue_2) (Variables|Default|GetMoveSpeed)) false false)))))))

(fn ConstructionScript
  (|CallParentFunction))