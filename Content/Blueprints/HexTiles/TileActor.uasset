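; An actor that occupies a hex on the HexMap, snapping to it in the editor and registering with it at runtime.
; The Construction Script finds the map by SnapCollision overlap, snaps only RootMesh to the hex point and stores HexPosition.
; BeginPlay disables that collision, registers with the game mode's CurrentHexMap and moves the scene root onto the snapped mesh.
; ChangePosition updates registration and HexPosition without moving the actor.
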(event EventBeginPlay
  (bind _rootmesh (Variables|Default|GetRootMesh))
  (Collision|SetCollisionEnabled (Variables|Default|GetSnapCollision) "NoCollision") ; We turn off the collsion, since we only use it in the construction script
  (Class|HexMap|RegisterActortoHex (Variables|/Script/HexGameFramework.HexGameFrameworkGameModeBase|GetCurrentHexMap (Utilities|GetHexGameMode)) (Variables|Default|GetHexPosition) self)
  (Transformation|SetWorldLocation (Variables|Default|GetDefaultSceneRoot) (Transformation|GetWorldLocation _rootmesh) false false)
  (Transformation|SetRelativeLocation _rootmesh "0, 0, 0" false false))

(fn ConstructionScript
  ;[1 1 1] Tile snapping and initial position setting
  (bind _outactors (Collision|ComponentOverlapActors (Variables|Default|GetSnapCollision) (Transformation|GetActorTransform) (Utilities|Array|MakeArray "ObjectTypeQuery2") "/Game/Blueprints/HexMap.HexMap_C"))
  (Transformation|SetWorldLocation (Variables|Default|GetRootMesh) (Class|HexMap|HexVectortoPoint (.AsHex%20Map (Utilities|Casting|CastToHexMap (Utilities|Array|Get(acopy) _outactors))) (Class|HexMap|PointtoHexVector (.AsHex%20Map (Utilities|Casting|CastToHexMap (Utilities|Array|Get(acopy) _outactors))) (Transformation|GetWorldLocation (Variables|Default|GetDefaultSceneRoot)))) false false)
  (Variables|Default|SetHexPosition (Class|HexMap|PointtoHexVector (.AsHex%20Map (Utilities|Casting|CastToHexMap (Utilities|Array|Get(acopy) _outactors))) (Transformation|GetWorldLocation (Variables|Default|GetDefaultSceneRoot)))))

(fn ChangePosition
  (params (NewPosition :type Hex%20Vector%20Structure))
  (bind _hexgamemode (Utilities|GetHexGameMode))
  (bind _self self)
  (bind _currenthexmap (Variables|/Script/HexGameFramework.HexGameFrameworkGameModeBase|GetCurrentHexMap _hexgamemode))
  (Class|HexMap|UnregisterActorfromHex _currenthexmap (Variables|Default|GetHexPosition) _self)
  (Class|HexMap|RegisterActortoHex _currenthexmap NewPosition _self)
  (Variables|Default|SetHexPosition NewPosition))