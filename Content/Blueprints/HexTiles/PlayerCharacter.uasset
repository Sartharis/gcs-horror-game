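; Player-controlled hex-tile character for a turn-based game, selectable only during its turn.
; A move order succeeds if it targets its own hex or finds a path on the game mode's current hex map, which it then follows.
; Finishing a move ends the turn and clears the controller's selection.
; Selection and turn events swap the root mesh's emissive material as color feedback.
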(event TurnActivateDelegate(Turn)
  (Rendering|Material|SetMaterial (Variables|Default|GetRootMesh) 0 "/Game/ColorEmissiveMaterial_Green.ColorEmissiveMaterial_Green"))

(event TurnEndDelegate(Turn)
  (Rendering|Material|SetMaterial (Variables|Default|GetRootMesh) 0 "/Game/ColorEmissiveMaterial_Red.ColorEmissiveMaterial_Red"))

(event EventOnMoveEnd
  (|CallParentFunction)
  (Class|TurnComponent|EndTurn (Variables|Default|GetTurn))
  (Default|UnselectAll (Utilities|GetPlayerTileController)))

(event EventOnSelected
  (Rendering|Material|SetMaterial (Variables|Default|GetRootMesh) 0 "/Game/ColorEmissiveMaterial_Yellow.ColorEmissiveMaterial_Yellow"))

(event EventOnUnselected
  (Rendering|Material|SetMaterial (Variables|Default|GetRootMesh) 0 "/Game/ColorEmissiveMaterial.ColorEmissiveMaterial"))

(fn ConstructionScript
  (|CallParentFunction))

(fn CanbeSelected
  (return (Class|TurnComponent|IsinTurn (Variables|Default|GetTurn))))

(fn OnMoveOrder
  (params (TargetHex :type Hex%20Vector%20Structure))
  (bind _hexgamemode (Utilities|GetHexGameMode))
  (bind _hexposition (Variables|Default|GetHexPosition))
  (bind _currenthexmap (Variables|/Script/HexGameFramework.HexGameFrameworkGameModeBase|GetCurrentHexMap _hexgamemode))
  (bind _returnvalue (Class|HexMap|GetPathBetweenHexes _currenthexmap _hexposition TargetHex))
  (if (Class|HexFunctionLibrary|EqualHexVectorHexVector _hexposition TargetHex)
    (return true)
    (elif (> (Utilities|Array|Length _returnvalue) 0)
      (CallFunction|MoveAlongPath _returnvalue)
      (return true)
      (else
        (return false)))))